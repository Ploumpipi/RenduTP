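; BP_Crystal is a collectible pickup that spins in place until a ThirdPersonCharacter overlaps it.
; On overlap it adds one to the character's Collectible count and destroys itself at once.
; Tick applies a fixed local rotation each frame, so spin speed depends on frame rate.
; An unconnected Timeline chain that would pull the crystal toward the player before destroying it never runs.
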(event EventTick
  (params (DeltaSeconds :type Float%20%28single-precision%29))
  (Transformation|AddActorLocalRotation "0,1.000000, 0" false false))

(event Collision|EventActorBeginOverlap
  (params (OtherActor :type Actor%20Object%20Reference))
  (bind _asthird_person_character (Utilities|Casting|CastToThirdPersonCharacter OtherActor))
  (Variables|/Game/ThirdPersonBP/Blueprints/ThirdPersonCharacter.ThirdPersonCharacter_C|SetCollectible _asthird_person_character (+ (Variables|/Game/ThirdPersonBP/Blueprints/ThirdPersonCharacter.ThirdPersonCharacter_C|GetCollectible _asthird_person_character) 1.0))
  (Actor|DestroyActor))

(event Collision|EventActorEndOverlap
  (params (OtherActor :type Actor%20Object%20Reference)))

(fn ConstructionScript)